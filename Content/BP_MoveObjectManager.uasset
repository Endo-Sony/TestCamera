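; A manager actor that moves tagged actors along a level spline and toggles the player's view to a spline camera.
; At BeginPlay it caches the default view target, the first "SprineCamera"-tagged actor and the BP_Spline component.
; MoveObject and MoveCamera feed the first "MoveTarget" actor or that camera into MoveAlongSpline, where a timeline sets location by spline distance.
; SwitchPlayerCamera swaps view targets between the two cameras.
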(event `self.ReceiveBeginPlay`
  (`self.Initialize`))

(event `MoveAlongSpline`
  (params (MoveActor :type "Actor Object Reference"))
  (bind _sprine (`self.Sprine`))
  (bind (_direction _rate) (`Timeline|MoveRate` :!via `PlayFromStart`)
    (:`Update`
      (`self.K2_SetActorLocation` MoveActor (`SplineComponent.GetLocationAtDistanceAlongSpline` _sprine (* _rate (`SplineComponent.GetSplineLength` _sprine)) "World") false false))))

(fn `Initialize`
  (set `self.PlayerDefaultCameraActor` (`Controller.GetViewTarget` (`GameplayStatics.GetPlayerController` 0)))
  (bind _outactors (`GameplayStatics.GetAllActorsOfClassWithTag` "/Script/Engine.Actor" "SprineCamera"))
  (set `self.SprineCameraActor` (`|GetArrayItem` _outactors))
  (bind _returnvalue (`GameplayStatics.GetActorOfClass` "/Game/BP_Spline.BP_Spline_C"))
  (set `self.Sprine` (`/Game/BP_Spline.Spline` _returnvalue)))

(fn `MoveCamera`
  (`self.MoveAlongSpline` (`self.SprineCameraActor`)))

(fn `MoveObject`
  (bind _outactors (`GameplayStatics.GetAllActorsWithTag` "MoveTarget"))
  (`self.MoveAlongSpline` (`|GetArrayItem` _outactors)))

(fn `SwitchPlayerCamera`
  (bind _returnvalue (`GameplayStatics.GetPlayerController` 0))
  (`KismetSystemLibrary.PrintString` "Switch PlayerCamera")
  (if (`self.IsSprineCamera`)
    (`PlayerController.SetViewTargetWithBlend` _returnvalue (`self.PlayerDefaultCameraActor`) 0.0 "VTBlend_Linear" 0.0 false)
    (set `self.IsSprineCamera` false)
    (else
      (`PlayerController.SetViewTargetWithBlend` _returnvalue (`self.SprineCameraActor`) 0.0 "VTBlend_Linear" 0.0 false)
      (set `self.IsSprineCamera` true))))

(fn `UserConstructionScript`)